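; Player Blueprint that turns its camera with the mouse and detects which object the player is looking at.
; MouseY also fires a Visibility line trace from the camera, skipping the game instance's ignore list and printing the hit actor's name.
; ClickableObject hits receive ReciveEyeTrack once LookOther is set, and a trace miss clears that flag.
; Helper functions for tag checks and click-timing resets are defined but never called here.
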(event `InputAxisKey|MouseX`
  (params (AxisValue :type "Float (single-precision)"))
  ;[1 0.1254 0.9859] 視線変更
  (`SceneComponent.K2_AddWorldRotation` (`self.Camera`) (`KismetMathLibrary.MakeRotator` 0.0 0.0 AxisValue) false false))

(event `InputAxisKey|MouseY`
  (params (AxisValue :type "Float (single-precision)"))
  (bind _camera (`self.Camera`))
  ;[1 0.1254 0.9859] 視線変更
  (`SceneComponent.K2_AddLocalRotation` _camera (`KismetMathLibrary.MakeRotator` 0.0 AxisValue) false false)
  ;[1 0.07345 0.7481] 視線の先の物を見分ける
  (bind _hitactor (`self.TraceUsingCamera` _camera _camera))
  (`KismetSystemLibrary.PrintString` (`KismetSystemLibrary.GetDisplayName` _hitactor))
  (bind _asclickable_object (cast `/Game/otsuka/BaseBluePrint/ClickableObject` _hitactor))
  (if (`self.LookOther`)
    (`/Game/otsuka/BaseBluePrint/ClickableObject.ReciveEyeTrack` _asclickable_object)
    (if true
      _)
    (else
      (set `self.LookOther` true))))

(fn `CheckTags`
  (params (self2 :type "ActorComponent Object Reference"))
  (returns (Item :type Name))
  ;[1 0.09391 0.814] ターゲットの判定
  (for _index (range (+ (`self.EndNum`) 1))
    (bind _item (`KismetArrayLibrary.Array_Get` (`self.TagName`) _index))
    (if (`ActorComponent.ComponentHasTag` self2 _item)
      (return _item)))
  (return _item))

(fn `GetActorName`
  (params (Object :type "Object Object Reference"))
  ;[1 0.04 0.04] アクタの名前の取得
  (bind _output_get (set `self.ActorName` (`KismetSystemLibrary.GetDisplayName` Object)))
  (switch `name` (`KismetStringLibrary.Conv_StringToName` _output_get)
    (:`Default`
      _)
    (:`Cube`
      _)
    (:`Case_0`
      _))
  (return))

(fn `InitMouseClickRelation`
  (bind _resettimenum (`self.ResetTimeNum`))
  ;[1 0 0.7692] 初期化
  (set `self.Clicked` false)
  (set `self.BarrageClick` false)
  (if (`self.Barraging`)
    (set `self.Time` _resettimenum)
    (set `self.Barraging` false)
    (else
      (set `self.Time` _resettimenum)))
  (return))

(fn `ResetClickTimeAndClickNum`
  ;[1 0.07151 0.8287] クリックしたときの時間と回数をリセットする
  (bind _output_get (set `self.Time` (+ (`self.Time`) 1)))
  (if (<= (`self.ResetTimeNum`) _output_get)
    (set `self.ClickNum` 0)
    (set `self.Time` 0))
  (return))

(fn `TraceUsingCamera`
  (params (self2 :type "SceneComponent Object Reference") (self3 :type "SceneComponent Object Reference"))
  (returns (HitActor :type "Actor Object Reference") (HitComponent :type "PrimitiveComponent Object Reference"))
  (bind _returnvalue (`SceneComponent.K2_GetComponentLocation` self2))
  ;[1 0.1363 0.8246] 視線の向きによる当たり判定
  (bind _asgame_instance_test (`self.GetThisGameInstance`))
  (bind (_outhit _returnvalue_2) (`KismetSystemLibrary.LineTraceSingle` _returnvalue (+ _returnvalue (* (`KismetMathLibrary.Conv_RotatorToVector` (`SceneComponent.K2_GetComponentRotation` self3)) 1500.0)) "TraceTypeQuery1" false (`/Game/otsuka/GameInstance_Test.ignoreActorList` _asgame_instance_test) "ForOneFrame"))
  (if (not _returnvalue_2)
    (set `self.LookOther` false))
  (bind (_bblockinghit _binitialoverlap _time _location _impactpoint _normal _impactnormal _physmat _hitactor _hitcomponent) (`GameplayStatics.BreakHitResult` _outhit))
  (return _hitactor _hitcomponent))

(fn `UserConstructionScript`)