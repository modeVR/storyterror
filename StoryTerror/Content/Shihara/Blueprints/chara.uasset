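; Blueprint "chara" that highlights the static mesh the player camera is looking at.
; Each Tick, it line-traces on Visibility from the camera along its forward vector, with debug drawing enabled.
; A static mesh hit gets Render Custom Depth enabled, and the previously stored component has it disabled.
; The last highlight persists when the trace misses or hits another component type.
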(event `self.ReceiveTick`
  (params (DeltaSeconds :type "Float (single-precision)"))
  (bind _returnvalue (`GameplayStatics.GetPlayerCameraManager` 0))
  (bind _hitcompornet (`self.Hitcompornet`))
  (bind _returnvalue_2 (`self.K2_GetActorLocation` _returnvalue))
  (bind (_outhit _returnvalue_3) (`KismetSystemLibrary.LineTraceSingle` :`Start` _returnvalue_2 :`End` (+ _returnvalue_2 (* (`self.GetActorForwardVector` _returnvalue) 1000.0)) :`TraceChannel` "TraceTypeQuery1" :`DrawDebugType` "ForDuration"))
  (if _returnvalue_3
    (bind `_asスタティックメッシュコンポーネント` (cast `StaticMeshComponent` (`.HitComponent` (`GameplayStatics.BreakHitResult` _outhit))))
    (`/Engine/EditorBlueprintResources/StandardMacros.IsValid` _hitcompornet
      (:`Is Valid`
        (`PrimitiveComponent.SetRenderCustomDepth` _hitcompornet false))
      (:`Is Not Valid`
        _))
    (set `self.Hitcompornet` `_asスタティックメッシュコンポーネント`)
    (`PrimitiveComponent.SetRenderCustomDepth` _hitcompornet true)))

(fn `UserConstructionScript`)