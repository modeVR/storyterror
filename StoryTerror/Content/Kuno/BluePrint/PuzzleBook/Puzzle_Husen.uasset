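; Puzzle book Husen actor that stays inactive until revealed, pairing a Paper2D sprite with an Icon child actor.
; On BeginPlay it hides the Icon, shows the "before" sprite and disables collision on itself and the child actor.
; The VisibleOn event reverses this, showing the Icon, swapping to the Husen sprite and enabling both collisions, with a leftover "Hello" debug print.
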(event `self.ReceiveBeginPlay`
  (`SceneComponent.SetVisibility` (`self.Icon`) false true)
  (`PaperSpriteComponent.SetSprite` (`self.PaperSprite`) "/Game/Kuno/BluePrint/PuzzleBook/png/husen_bef_Sprite.husen_bef_Sprite")
  (`self.SetActorEnableCollision` (`ChildActorComponent.ChildActor` (`self.Icon`)) false)
  (`self.SetActorEnableCollision` self false))

(event `VisibleOn`
  (`SceneComponent.SetVisibility` (`self.Icon`) true true)
  (`PaperSpriteComponent.SetSprite` (`self.PaperSprite`) "/Game/Kuno/BluePrint/PuzzleBook/png/husen_Sprite.husen_Sprite")
  (`KismetSystemLibrary.PrintString` "Hello")
  (`self.SetActorEnableCollision` (`ChildActorComponent.ChildActor` (`self.Icon`)) true)
  (`self.SetActorEnableCollision` self true))

(fn `UserConstructionScript`)