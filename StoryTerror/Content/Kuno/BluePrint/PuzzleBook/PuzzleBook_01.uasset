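; Puzzle book actor where sticky notes (Husen) are dragged onto hit fields and checked for correct placement.
; BeginPlay gathers tagged child actors and assigns their ID numbers from arrays.
; DragAction moves dragged icons to the line-trace point, otherwise snapping them to a hit field or returning them to their start.
; DragEndAction re-runs that pass after a brief delay; number matches only print debug messages.
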(event `self.ReceiveBeginPlay`
  ;[1 1 1] 配列内の情報を子アクターに格納
  (bind _output_get (set `self.ary_child` (`self.GetComponentsByTag` "/Script/Engine.ChildActorComponent" "Husen")))
  (bind _output_get_2 (set `self.ary_hitFieldActor` (`self.GetComponentsByTag` "/Script/Engine.ChildActorComponent" "FIeld")))
  (for _index (range (`KismetArrayLibrary.Array_Length` _output_get_2))
    (bind _aspuzzle_husen_hit_point (cast `/Game/Kuno/BluePrint/PuzzleBook/Puzzle_HusenHitPoint` (`ChildActorComponent.ChildActor` (`KismetArrayLibrary.Array_Get` _output_get_2 _index))))
    (set `/Game/Kuno/BluePrint/PuzzleBook/Puzzle_HusenHitPoint.num_HitNumber` (`KismetArrayLibrary.Array_Get` (`self.ary_HitNumber`) _index) _aspuzzle_husen_hit_point)
    (for _index_2 (range (`KismetArrayLibrary.Array_Length` _output_get))
      (bind _aspuzzle_husen (cast `/Game/Kuno/BluePrint/PuzzleBook/Puzzle_Husen` (`ChildActorComponent.ChildActor` (`KismetArrayLibrary.Array_Get` _output_get _index_2))))
      (set `/Game/Kuno/BluePrint/PuzzleBook/Puzzle_Husen.num_itemNumber` (`KismetArrayLibrary.Array_Get` (`self.ary_IconNumber`) _index_2) _aspuzzle_husen))))

(event `self.DragAction`
  (bind _ary_child (`self.ary_child`))
  (bind _ary_hitfieldactor (`self.ary_hitFieldActor`))
  ;[1 1 1] 配列内に格納したふせんの移動処理
  (for _index (range (`KismetArrayLibrary.Array_Length` _ary_child)) :!label _label
    (bind _aspuzzle_husen (cast `/Game/Kuno/BluePrint/PuzzleBook/Puzzle_Husen` (`ChildActorComponent.ChildActor` (`KismetArrayLibrary.Array_Get` _ary_child _index))))
    (bind _childactor (`ChildActorComponent.ChildActor` (`/Game/Kuno/BluePrint/PuzzleBook/Puzzle_Husen.Icon` _aspuzzle_husen)))
    (bind _ashusen_icon (cast `/Game/Kuno/BluePrint/PuzzleBook/HusenIcon` _childactor :!pure true))
    (if (`/Game/Kuno/BluePrint/PuzzleBook/HusenIcon.flg_drag` _ashusen_icon)
      (`self.K2_SetActorLocation` _childactor (`KismetMathLibrary.MakeVector` (.x (`self.LineHitPoint`)) (.y (`self.LineHitPoint`)) (- (.z (`self.LineHitPoint`)) -1.0)) false false)
      (else
        ;[1 1 1] ドロップ後の吸着と正誤判定
        (for _index_2 (range (`KismetArrayLibrary.Array_Length` _ary_hitfieldactor))
          (bind _childactor_2 (`ChildActorComponent.ChildActor` (`KismetArrayLibrary.Array_Get` _ary_hitfieldactor _index_2)))
          (bind _aspuzzle_husen_hit_point (cast `/Game/Kuno/BluePrint/PuzzleBook/Puzzle_HusenHitPoint` _childactor_2))
          (if (`/Game/Kuno/BluePrint/PuzzleBook/Puzzle_HusenHitPoint.flg_hit` _aspuzzle_husen_hit_point)
            (bind _pos_first (`/Game/Kuno/BluePrint/PuzzleBook/HusenIcon.pos_first` _ashusen_icon))
            (if (== (`self.K2_GetActorLocation` _ashusen_icon) _pos_first)
              (`self.K2_SetActorLocation` _childactor _pos_first false false :!label _label_2)
              (else
                (`self.K2_SetActorLocation` _childactor (`self.K2_GetActorLocation` _childactor_2) false false)
                (if (== (`/Game/Kuno/BluePrint/PuzzleBook/Puzzle_Husen.num_itemNumber` _aspuzzle_husen) (`/Game/Kuno/BluePrint/PuzzleBook/Puzzle_HusenHitPoint.num_HitNumber` _aspuzzle_husen_hit_point))
                  (`KismetSystemLibrary.PrintString` "OK!!")
                  (else
                    (`KismetSystemLibrary.PrintString` "敗北者に塩")))))
            (else
              (goto _label_2))))))))

(event `self.DragEndAction`
  ;[1 1 1] 配列内に格納したふせんの移動処理
  (`KismetSystemLibrary.Delay` 0.01)
  (goto _label))

(fn `UserConstructionScript`)