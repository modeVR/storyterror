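; HusenIcon is a draggable paper-sprite icon for the puzzle book, spawned under a Puzzle_Husen actor.
; On BeginPlay it stores its starting location and picks its sprite from an array using the owning Puzzle_Husen's item number.
; Drag start and end events toggle a drag flag and switch sprite collision between Overlap and Block; the movement itself is not handled in these graphs.
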(event `self.ReceiveBeginPlay`
  (set `self.pos_first` (`SceneComponent.K2_GetComponentLocation` (`self.PaperSprite`)))
  (bind _aspuzzle_husen (cast `/Game/Kuno/BluePrint/PuzzleBook/Puzzle_Husen` (`ActorComponent.GetOwner` (`self.GetParentComponent`))))
  (`PaperSpriteComponent.SetSprite` (`self.PaperSprite`) (`KismetArrayLibrary.Array_Get` (`self.Sprite`) (`/Game/Kuno/BluePrint/PuzzleBook/Puzzle_Husen.num_itemNumber` _aspuzzle_husen))))

(event `self.DragStartAction`
  (set `self.flg_drag` true)
  (`PrimitiveComponent.SetCollisionResponseToAllChannels` (`self.PaperSprite`) "ECR_Overlap"))

(event `self.DragEndAction`
  (set `self.flg_drag` false)
  (`PrimitiveComponent.SetCollisionResponseToAllChannels` (`self.PaperSprite`) "ECR_Block")
  (`KismetSystemLibrary.PrintString` "www"))

(fn `UserConstructionScript`
  (`parent.UserConstructionScript`))