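; DAD is a draggable actor that follows the player's view horizontally while keeping a fixed height.
; BeginPlay records the root's starting location and its Z height.
; Each DragAction call moves the actor with sweep to the X and Y of a point 25 units ahead of the BP_player_DAD camera, at the stored Z.
; The saved starting location goes unused in these graphs.
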(event `self.ReceiveBeginPlay`
  (bind _returnvalue (`SceneComponent.K2_GetComponentLocation` (`self.Root`)))
  (set `self.pos_y` (.z _returnvalue))
  (set `self.pos_first` _returnvalue))

(event `self.DragAction`
  (bind _camera (`/Game/Kuno/BluePrint/BP_player_DAD.Camera` (cast `/Game/Kuno/BluePrint/BP_player_DAD` (`GameplayStatics.GetPlayerCharacter` 0) :!pure true)))
  (`self.K2_SetActorLocation` (`KismetMathLibrary.MakeVector` (.x (+ (`SceneComponent.K2_GetComponentLocation` _camera) (* (`KismetMathLibrary.GetForwardVector` (`SceneComponent.K2_GetComponentRotation` _camera)) 25.0))) (.y (+ (`SceneComponent.K2_GetComponentLocation` _camera) (* (`KismetMathLibrary.GetForwardVector` (`SceneComponent.K2_GetComponentRotation` _camera)) 25.0))) (`self.pos_y`)) true))

(fn `UserConstructionScript`
  (`parent.UserConstructionScript`))