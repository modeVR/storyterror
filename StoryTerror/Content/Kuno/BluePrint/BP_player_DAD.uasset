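; Player Blueprint that turns the camera with the mouse, interacts with looked-at objects and breaks mirrors.
; The MouseY axis event traces from the camera, sending eye-track notices and hit points to ClickableObjects after a one-update LookOther gate.
; On DestructibleActors, each fresh left click advances a damage material until enough clicks shatter it and start a destroy timer.
; Tick runs a shorter camera trace, skipping GameInstance-listed actors, to outline static meshes through custom depth.
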(event `InputAxisKey|MouseX`
  (params (AxisValue :type "Float (single-precision)"))
  ;[1 0.1254 0.9859] 視線変更
  (`SceneComponent.K2_AddWorldRotation` (`self.Camera`) (`KismetMathLibrary.MakeRotator` 0.0 0.0 AxisValue) false false))

(event `InputAxisKey|MouseY`
  (params (AxisValue :type "Float (single-precision)"))
  (bind _destructcount (`self.DestructCount`))
  (bind _camera (`self.Camera`))
  ;[1 0.1254 0.9859] 視線変更
  (`SceneComponent.K2_AddLocalRotation` _camera (`KismetMathLibrary.MakeRotator` 0.0 AxisValue) false false)
  ;[1 0.07345 0.7481] 視線の先の物を見分ける
  (bind (_hitactor _hitcomponent _hitlocation _impactdir) (`self.TraceUsingCamera` _camera _camera))
  (bind _asclickable_object (cast `/Game/otsuka/BaseBluePrint/ClickableObject` _hitactor)
    (:`then`
      (if (`self.LookOther`)
        (`/Game/otsuka/BaseBluePrint/ClickableObject.ReciveEyeTrack` _asclickable_object)
        (set `/Game/otsuka/BaseBluePrint/ClickableObject.LineHitPoint` _hitlocation _asclickable_object)
        (else
          (set `self.LookOther` true))))
    (:`CastFailed`
      (bind _asdestructible_actor (cast `DestructibleActor` _hitactor))
      (bind _output_get (set `self.DestructibleComponent` _asdestructible_actor))
      ;[1 0.1379 0.7634] 鏡が壊れる
      (if (`PlayerController.IsInputKeyDown` (`GameplayStatics.GetPlayerController` 0) "LeftMouseButton")
        (if (`self.Clicked`)
          (bind _destructiblecomponent (`DestructibleActor.DestructibleComponent` _output_get))
          (`PrimitiveComponent.SetMaterial` _destructiblecomponent 0 (`KismetArrayLibrary.Array_Get` (`self.Materials`) _destructcount))
          (bind _output_get_2 (set `self.DestructCount` (+ _destructcount 1)))
          (set `self.Clicked` false)
          (if (>= _output_get_2 4)
            (`DestructibleComponent.ApplyDamage` _destructiblecomponent 1.0 _hitlocation _impactdir 50.0)
            (`KismetSystemLibrary.K2_SetTimerDelegate` (delegate `Destroy`) (`self.DestructibleComponentDestroyTimer`))))
        (else
          (set `self.Clicked` true))))))

(event `Destroy`
  ;[1 0.1379 0.7634] 鏡が壊れる
  (`self.K2_DestroyActor` (`self.DestructibleComponent`)))

(event `self.ReceiveTick`
  (params (DeltaSeconds :type "Float (single-precision)"))
  (bind _returnvalue (`GameplayStatics.GetPlayerCameraManager` 0))
  (bind _hit_compornet (`self.Hit Compornet`))
  (bind _returnvalue_2 (`self.K2_GetActorLocation` _returnvalue))
  ;[1 1 1] OutLine表示
  (bind _asgi_game_instance (cast `/Game/otsuka/GI_GameInstance` (`GameplayStatics.GetGameInstance`)))
  (bind (_outhit _returnvalue_3) (`KismetSystemLibrary.LineTraceSingle` _returnvalue_2 (+ _returnvalue_2 (* (`self.GetActorForwardVector` _returnvalue) 1000.0)) "TraceTypeQuery1" false (`/Game/otsuka/GI_GameInstance.ignoreActorList` _asgi_game_instance)))
  (if _returnvalue_3
    (bind `_asスタティックメッシュコンポーネント` (cast `StaticMeshComponent` (`.HitComponent` (`GameplayStatics.BreakHitResult` _outhit))))
    (`/Engine/EditorBlueprintResources/StandardMacros.IsValid` _hit_compornet
      (:`Is Valid`
        (`PrimitiveComponent.SetRenderCustomDepth` _hit_compornet false))
      (:`Is Not Valid`
        _))
    (set `self.Hit Compornet` `_asスタティックメッシュコンポーネント`)
    (`PrimitiveComponent.SetRenderCustomDepth` _hit_compornet true)))

(fn `TraceUsingCamera`
  (params (self2 :type "SceneComponent Object Reference") (self3 :type "SceneComponent Object Reference"))
  (returns (HitActor :type "Actor Object Reference") (HitComponent :type "PrimitiveComponent Object Reference") (HitLocation :type "Vector Structure") (ImpactDir :type "Vector Structure"))
  (bind _returnvalue (`SceneComponent.K2_GetComponentLocation` self2))
  ;[1 0.1363 0.8246] 視線の向きによる当たり判定
  (bind (_outhit _returnvalue_2) (`KismetSystemLibrary.LineTraceSingle` :`Start` _returnvalue :`End` (+ _returnvalue (* (`KismetMathLibrary.GetForwardVector` (`SceneComponent.K2_GetComponentRotation` self3)) 2500.0)) :`TraceChannel` "TraceTypeQuery1" :`DrawDebugType` "ForOneFrame"))
  (if (not _returnvalue_2)
    (set `self.LookOther` false))
  (bind (_bblockinghit _binitialoverlap _time _location _impactpoint _normal _impactnormal _physmat _hitactor _hitcomponent) (`GameplayStatics.BreakHitResult` _outhit))
  (return _hitactor _hitcomponent _impactpoint _impactnormal))

(fn `UserConstructionScript`)