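; Practice actor for eye-tracked clicking that shows a text prompt and rotates its mesh by a fixed step per left click.
; The first ReciveEyeTrack call shows the text; later calls poll the mouse, using a Pressing flag to fire Action once per press.
; EndText toggles text visibility without resetting TrackTextVisibility.
; CheckClick duplicates the press check without triggering Action and is not called here.
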(event `self.ReciveEyeTrack`
  (if (`self.TrackTextVisibility`)
    ;[1 0.04638 0.6841] クリックの判定
    (if (`PlayerController.IsInputKeyDown` (`GameplayStatics.GetPlayerController` 0) "LeftMouseButton")
      (if (not (`self.Pressing`))
        (set `self.Pressing` true)
        (`self.Action`))
      (else
        (set `self.Pressing` false)))
    (else
      (`SceneComponent.ToggleVisibility` (`self.TextRender`) true)
      (set `self.TrackTextVisibility` true))))

(event `self.Action`
  (`SceneComponent.K2_AddWorldRotation` (`self.StaticMesh`) (struct :`Yaw` 20.0) false false))

(fn `CheckClick`
  ;[1 0.04638 0.6841] クリックの判定
  (if (`PlayerController.IsInputKeyDown` (`GameplayStatics.GetPlayerController` 0) "LeftMouseButton")
    (if (not (`self.Pressing`))
      (set `self.Pressing` true)
      (return))
    (else
      (set `self.Pressing` false))))

(fn `EndText`
  (`SceneComponent.ToggleVisibility` (`self.TextRender`) false))

(fn `UserConstructionScript`
  (`parent.UserConstructionScript`))