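; BarragiObject is an eye-tracked actor that starts rotating when the player rapidly clicks the left mouse button.
; Each ReciveEyeTrack call after the first polls the button, using a Pressing flag to count each press once.
; Five clicks set Barraging, while calls without input advance a counter that clears clicks at ResetTimeNum.
; Once Barraging is set, every call rotates the mesh and bypasses the reset, so the state latches.
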(event `self.ReciveEyeTrack`
  (bind _barraging (`self.Barraging`))
  (if (`self.SeenMe`)
    (if (`PlayerController.IsInputKeyDown` (`GameplayStatics.GetPlayerController` 0) "LeftMouseButton")
      (if _barraging
        (`self.Action` :!label _label)
        (elif (not (`self.Pressing`))
          (`self.CheckClickNumber`)))
      (elif _barraging
        (goto _label)
        (else
          (`self.ResetClickNumber`)
          (set `self.Pressing` false))))
    (else
      (set `self.SeenMe` true))))

(event `self.Action`
  (`SceneComponent.K2_AddWorldRotation` (`self.StaticMesh`) (struct :`Pitch` 2.0 :`Yaw` 2.0) false false))

(fn `CheckClickNumber`
  ;[1 0 0.7931] クリックした数による連打の成功判定
  (bind _output_get (set `self.ClickNum` (+ (`self.ClickNum`) 1)))
  (set `self.Time` 0)
  (set `self.Barraging` (<= 5 _output_get))
  (set `self.Pressing` true)
  (return))

(fn `ResetClickNumber`
  ;[1 0.01025 0.6822] 時間経過によっての値の初期化
  (bind _output_get (set `self.Time` (+ (`self.Time`) 1)))
  (if (<= (`self.ResetTimeNum`) _output_get)
    (set `self.ClickNum` 0)
    (set `self.Time` 0)
    (set `self.Barraging` false))
  (return))

(fn `UserConstructionScript`
  (`parent.UserConstructionScript`))