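; Practice pressable object that responds to eye-tracking notifications by revealing a text prompt.
; The first ReciveEyeTrack call toggles the TextRender's visibility and sets TrackTextVisibility; later calls invoke Action while the left mouse button is held.
; EndText toggles the text again without clearing the flag in this graph.
; Action is not defined here, and the default events are empty.
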(event `self.ReciveEyeTrack`
  (if (`self.TrackTextVisibility`)
    (if (`PlayerController.IsInputKeyDown` (`GameplayStatics.GetPlayerController` 0) "LeftMouseButton")
      (`self.Action`))
    (else
      (`SceneComponent.ToggleVisibility` (`self.TextRender`) true)
      (set `self.TrackTextVisibility` true))))

(fn `EndText`
  (`SceneComponent.ToggleVisibility` (`self.TextRender`) false))

(fn `UserConstructionScript`
  (`parent.UserConstructionScript`))