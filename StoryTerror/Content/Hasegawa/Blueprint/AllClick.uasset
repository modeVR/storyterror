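; AllClick is a gaze-target actor whose static mesh rotates a fixed step when triggered by left-mouse input.
; ReciveEyeTrack matches mesh component tags against TagName to select Press, Click or Barrage Click handling.
; Each mode polls whether the button is held, using call counters rather than click events: Press waits for LongTime, while Barrage Click's count resets on release.
; ReciveClickEvent is empty.
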(event `self.Action`
  (`SceneComponent.K2_AddWorldRotation` (`self.StaticMesh`) (struct :`Yaw` 20.0) false false))

(event `self.ReciveEyeTrack`
  (bind _nowtime (`self.NowTime`))
  (bind _nowtime_2 (`self.NowTime`))
  (bind _clicknum (`self.ClickNum`))
  (bind _nowtime_3 (`self.NowTime`))
  (bind _returnvalue (`PlayerController.IsInputKeyDown` (`GameplayStatics.GetPlayerController` 0) "LeftMouseButton"))
  (for _index (range (+ (`self.EndNum`) 1))
    (bind _item (`KismetArrayLibrary.Array_Get` (`self.TagName`) _index))
    ;[1 0.07345 0.7481] 視線の先の物を見分ける
    (if (`ActorComponent.ComponentHasTag` (`self.StaticMesh`) _item)
      (switch `name` _item
        (:`Press`
          ;[1 0.05507 0.8517] 長押しの処理
          (if _returnvalue
            (if (>= _nowtime (`self.LongTime`))
              (`self.Action`)
              (else
                (set `self.NowTime` (+ _nowtime 1.0))))
            (else
              (set `self.NowTime` 0.0 :!label _label))))
        (:`Click`
          (if _returnvalue
            (if (<= _nowtime_2 (`self.MinTime`))
              (`self.Action`)
              (else
                (set `self.NowTime` (+ _nowtime_2 1.0))))
            (else
              (goto _label))))
        (:`BarrageClick`
          (if _returnvalue
            (if (<= _nowtime_3 (`self.MinTime`))
              (if (>= _clicknum 5)
                (`self.Action`)
                (else
                  (set `self.ClickNum` (+ _clicknum 1))))
              (else
                (set `self.NowTime` (+ _nowtime_3 1.0))))
            (else
              (set `self.ClickNum` 0)
              (goto _label))))))))

(event `self.ReciveClickEvent`)

(fn `UserConstructionScript`
  (`parent.UserConstructionScript`))