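; ClickingObject is an actor Blueprint that reacts to an eye-tracking event by rotating its static mesh.
; Each ReciveEyeTrack call runs CheckClick, then Action, which adds a fixed world rotation step to the mesh.
; CheckClick polls the left mouse button into a Pressing flag, but the rotation runs regardless of that flag.
; BeginPlay, overlap and Tick are empty, so all behavior depends on that event being called.
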(event `self.ReciveEyeTrack`
  (`self.CheckClick`)
  (`self.Action`))

(event `self.Action`
  (`SceneComponent.K2_AddWorldRotation` (`self.StaticMesh`) (struct :`Yaw` 20.0) false false))

(fn `CheckClick`
  ;[1 0.04638 0.6841] クリックの判定
  (if (`PlayerController.IsInputKeyDown` (`GameplayStatics.GetPlayerController` 0) "LeftMouseButton")
    (if (not (`self.Pressing`))
      (set `self.Pressing` true))
    (else
      (set `self.Pressing` false)))
  (return))

(fn `UserConstructionScript`
  (`parent.UserConstructionScript`))