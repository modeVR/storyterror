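; Icon item actor that can be dragged with the mouse once activated.
; GetItem turns the icon material blue and enables it to respond to ReciveEyeTrack.
; While left mouse is held during that event, mouse deltas move the static mesh along world Y and Z.
; Drag speed scales with the square root of distance to Player via nested roots, and is printed for debugging.
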(event `self.ReciveEyeTrack`
  (bind _returnvalue (`GameplayStatics.GetPlayerController` 0))
  (bind _movement (`self.movement`))
  (bind (_deltax _deltay) (`PlayerController.GetInputMouseDelta` _returnvalue))
  (if (`self.OnActive`)
    (if (`PlayerController.IsInputKeyDown` _returnvalue "LeftMouseButton")
      (`self.The distance between the three points`)
      (`SceneComponent.K2_AddWorldTransform` (`self.StaticMesh`) (`KismetMathLibrary.MakeTransform` (`KismetMathLibrary.MakeVector` 0.0 (* _deltax _movement) (* _deltay _movement)) (struct) (1.0 1.0 1.0)) false false))))

(fn `GetItem`
  (`PrimitiveComponent.SetMaterial` (`self.Icom`) 0 "/Game/Material/Blue.Blue")
  (set `self.OnActive` true))

(fn `The distance between the three points`
  (bind (_returnvalue_x _returnvalue_y _returnvalue_z) (`KismetMathLibrary.BreakVector` (`self.K2_GetActorLocation`)))
  (bind (_returnvalue_x_2 _returnvalue_y_2 _returnvalue_z_2) (`KismetMathLibrary.BreakVector` (`self.K2_GetActorLocation` (`self.player`))))
  (bind _returnvalue (`KismetMathLibrary.Sqrt` (`KismetMathLibrary.Sqrt` (`KismetMathLibrary.Sqrt` (+ (`KismetMathLibrary.MultiplyMultiply_FloatFloat` (- _returnvalue_x _returnvalue_x_2) 2.0) (`KismetMathLibrary.MultiplyMultiply_FloatFloat` (- _returnvalue_y _returnvalue_y_2) 2.0) (`KismetMathLibrary.MultiplyMultiply_FloatFloat` (- _returnvalue_z _returnvalue_z_2) 2.0))))))
  (bind _output_get (set `self.movement` (* _returnvalue (/ _returnvalue 3.0))))
  (`KismetSystemLibrary.PrintString` (`KismetStringLibrary.Conv_DoubleToString` _output_get))
  (return))

(fn `UserConstructionScript`
  (`parent.UserConstructionScript`))