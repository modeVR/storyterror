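; An item actor with Icon and Postit components that lets the player move the Icon once it is picked up.
; GetItem turns both components red and sets it active, enabling the externally triggered Action event.
; Action offsets the Icon locally using mouse delta for Y-up plane movement (X and Z) and Up/Down keys for fixed Y steps.
; Mouse movement scales nonlinearly with Icon-to-Player distance divided by Speed, with the factor printed for debugging.
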(event `/Game/otsuka/BaseBluePrint/ClickableObject.Action`
  (bind _returnvalue (`GameplayStatics.GetPlayerController` 0))
  (bind _movement (`self.movement`))
  (bind (_deltax _deltay) (`PlayerController.GetInputMouseDelta` _returnvalue))
  (if (`self.OnActive`)
    (`self.The distance between the three points`)
    (if (`PlayerController.IsInputKeyDown` _returnvalue "Up")
      (set `self.moveX` 1.0)
      (elif (`PlayerController.IsInputKeyDown` _returnvalue "Down")
        (set `self.moveX` -1.0)
        (else
          (set `self.moveX` 0.0))))
    (`SceneComponent.K2_AddLocalTransform` (`self.Icon`) (`KismetMathLibrary.MakeTransform` (`KismetMathLibrary.MakeVector` (* _deltax _movement) (`self.moveX`) (* _deltay _movement))) false false)))

(fn `GetItem`
  (`PrimitiveComponent.SetMaterial` (`self.Icon`) 0 "/Game/Hasegawa/Material/Red.Red")
  (set `self.OnActive` true)
  (`PrimitiveComponent.SetMaterial` (`self.Postit`) 0 "/Game/Hasegawa/Material/Red.Red"))

(fn `The distance between the three points`
  (bind (_returnvalue_x _returnvalue_y _returnvalue_z) (`KismetMathLibrary.BreakVector` (`self.K2_GetActorLocation` (`self.Player`))))
  (bind (_returnvalue_x_2 _returnvalue_y_2 _returnvalue_z_2) (`KismetMathLibrary.BreakVector` (`SceneComponent.K2_GetComponentLocation` (`self.Icon`))))
  (bind _returnvalue (`KismetMathLibrary.Sqrt` (`KismetMathLibrary.Sqrt` (+ (`KismetMathLibrary.MultiplyMultiply_FloatFloat` (- _returnvalue_x_2 _returnvalue_x) 2.0) (`KismetMathLibrary.MultiplyMultiply_FloatFloat` (- _returnvalue_y_2 _returnvalue_y) 2.0) (`KismetMathLibrary.MultiplyMultiply_FloatFloat` (- _returnvalue_z_2 _returnvalue_z) 2.0)))))
  (bind _output_get (set `self.movement` (* (`KismetMathLibrary.Sqrt` _returnvalue) (/ _returnvalue (`self.Speed`)))))
  (`KismetSystemLibrary.PrintString` (`KismetStringLibrary.Conv_DoubleToString` _output_get))
  (return))

(fn `UserConstructionScript`
  (`parent.UserConstructionScript`))