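; ItemIcon is an item icon actor that the player can drag with the mouse once the item is obtained.
; GetItem turns the icon blue and sets OnActive, enabling the ReciveEyeTrack event.
; While active, that event turns the icon brown and moves StaticMesh along world Y and Z by mouse delta scaled by Movement while left mouse is held.
; Otherwise, it restores the blue material.
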(event `self.ReciveEyeTrack`
  (bind _returnvalue (`GameplayStatics.GetPlayerController` 0))
  (bind _movement (`self.movement`))
  (bind (_deltax _deltay) (`PlayerController.GetInputMouseDelta` _returnvalue))
  (if (`self.OnActive`)
    (if (`PlayerController.IsInputKeyDown` _returnvalue "LeftMouseButton")
      (`PrimitiveComponent.SetMaterial` (`self.Icom`) 0 "/Game/Material/Brown.Brown")
      (`SceneComponent.K2_AddWorldTransform` (`self.StaticMesh`) (`KismetMathLibrary.MakeTransform` (`KismetMathLibrary.MakeVector` 0.0 (* _deltax _movement) (* _deltay _movement))) false false)
      (else
        (`PrimitiveComponent.SetMaterial` (`self.Icom`) 0 "/Game/Material/Blue.Blue")))))

(fn `GetItem`
  (`PrimitiveComponent.SetMaterial` (`self.Icom`) 0 "/Game/Material/Blue.Blue")
  (set `self.OnActive` true))

(fn `UserConstructionScript`
  (`parent.UserConstructionScript`))