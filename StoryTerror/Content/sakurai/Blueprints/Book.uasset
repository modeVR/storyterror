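; Interactive book actor that, on a right-click during an eye-track event, moves closer and opens to reveal floating text.
; A Pressing flag makes each click fire once, starting the MoveBook timeline that drives mesh location and rotation.
; Its completion starts OpenBook, which swings the left pieces with an offset correction, hides the spine, reveals text after a short delay, then notifies the level via EVOpenBookToLevel.
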(event `self.ReciveEyeTrack`
  ;[1 0.04638 0.6841] クリックの判定
  (if (`PlayerController.IsInputKeyDown` (`GameplayStatics.GetPlayerController` 0) "RightMouseButton")
    (if (not (`self.Pressing`))
      (set `self.Pressing` true)
      (`self.Action`))
    (else
      (set `self.Pressing` false))))

(event `self.Action`
  ;[1 1 1] 本の座標更新と向きの変更
  (bind (_direction _movingbookrotation _bookrotation _movebook) (`Timeline|MoveBook` :`NewTime` 0.0) ; 本が近くまで来る
    (:`Update`
      (`SceneComponent.K2_SetRelativeLocation` (`self.Mesh`) _movebook false false)
      (`SceneComponent.K2_SetRelativeRotation` (`self.Mesh`) (`KismetMathLibrary.MakeRotator` _movingbookrotation 0.0 _bookrotation) false false))
    (:`Finished`
      ;[1 1 1] 移動が終わり次第、本が開くアニメーションがスタート
      (bind (_direction_2 _bookopen _openbooklocation) (`Timeline|OpenBook`) ; 本が開く、位置を修正、文字を浮かべる
        (:`Update`
          (`SceneComponent.K2_SetRelativeLocation` (`self.BookLeftMiddle`) _openbooklocation false false)
          (`SceneComponent.K2_SetRelativeLocation` (`self.BookLeftUnder`) _openbooklocation false false) ; 座標が合わないので多少修正を入れる
          (`SceneComponent.K2_SetRelativeRotation` (`self.BookLeftMiddle`) (`KismetMathLibrary.MakeRotator` 0.0 _bookopen) false false)
          (`SceneComponent.K2_SetRelativeRotation` (`self.BookLeftUnder`) (`KismetMathLibrary.MakeRotator` 0.0 _bookopen) false false)
          (`SceneComponent.SetVisibility` (`self.BookBack`) false false) ; 背が残ったままになるので見た目上は消しておく
          (`KismetSystemLibrary.Delay` 0.2)
          (`SceneComponent.SetVisibility` (`self.ソウダガツオくん`) true false)
          (`SceneComponent.SetVisibility` (`self.そうだよ`) true false))
        (:`Finished`
          (`self.EVOpenBookToLevel`))))))

(event `self.ReceiveBeginPlay`
  (`AddComponent|Particle System Component_0`))

(fn `UserConstructionScript`
  (`parent.UserConstructionScript`))